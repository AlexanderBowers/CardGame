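; BP_SubtractToggle is a clickable toggle actor that flips its Active state and notifies the BP_JudgeController found at BeginPlay.
; Each click swaps material slot 0 on the static mesh children of its root between CardOutline when active and CardBase when inactive.
; The Judge's ToggleMessage fires inside both mesh loops, so it runs once per static mesh rather than once per click.
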(event `self.ReceiveBeginPlay`
  (add `self.OnClicked` (delegate `OnClicked_Event`))
  (bind _returnvalue (`GameplayStatics.GetActorOfClass` "/Game/BP_JudgeController.BP_JudgeController_C"))
  (set `self.Judge` _returnvalue))

(event `OnClicked_Event` :!signature `self.OnClicked`
  (params (TouchedActor :type "Actor Object Reference") (ButtonPressed :type "Key Structure" :default "None"))
  (`KismetSystemLibrary.PrintText` "Working!")
  (bind _output_get (set `self.bActive` (not (`self.bActive`))))
  (if _output_get
    (for _array_element (`SceneComponent.GetChildrenComponents` (`self.DefaultSceneRoot`) true)
      (bind _asstatic_mesh_component (cast `StaticMeshComponent` _array_element))
      (`PrimitiveComponent.SetMaterial` _asstatic_mesh_component 0 "/Game/Materials/CardOutline.CardOutline")
      (message `/Game/BPI_PlayerJudge.Toggle` (`self.Judge`) :!label _label))
    (else
      (for _array_element_2 (`SceneComponent.GetChildrenComponents` (`self.DefaultSceneRoot`) true)
        (bind _asstatic_mesh_component_2 (cast `StaticMeshComponent` _array_element_2))
        (`PrimitiveComponent.SetMaterial` _asstatic_mesh_component_2 0 "/Game/Materials/CardBase.CardBase")
        (goto _label)))))

(fn `UserConstructionScript`)