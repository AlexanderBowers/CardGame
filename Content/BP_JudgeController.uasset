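; BP_JudgeController acts as the card dealer, handling DealCard requests from player controllers.
; If the requester matches Player1, it spawns a BP_Card at the P1 transform, assigns the owning player and a random value, and sets the card's text.
; Only Player1 is handled: Player2 is unused, and any other requester or an invalid spawn just prints debug text.
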(event `/Game/BPI_PlayerJudge.Deal Card`
  (params (PlayerController :type "/Game/BP_CardPlayerController Object Reference"))
  (bind _player1 (`self.Player1`))
  (`KismetSystemLibrary.PrintText` "Judge received Event Deal Card")
  (if (== PlayerController _player1)
    (bind _returnvalue (`|SpawnActorFromClass` "/Game/BP_Card.BP_Card_C" (`SceneComponent.K2_GetComponentToWorld` (`self.P1`)) "Undefined" "MultiplyWithRoot" null null))
    (`/Engine/EditorBlueprintResources/StandardMacros.IsValid` _returnvalue
      (:`Is Valid`
        (set `Card.Player` PlayerController _returnvalue)
        (bind _output_get (set `Card.value` (`KismetMathLibrary.RandomIntegerInRange` 1 10) _returnvalue))
        (`TextRenderComponent.K2_SetText` (`/Game/BP_Card.TextValue` _returnvalue) (`KismetTextLibrary.Conv_IntToText` _output_get)))
      (:`Is Not Valid`
        (`KismetSystemLibrary.PrintText` "Card Not valid!")))
    (else
      (`KismetSystemLibrary.PrintText` "Player 1 branch failed!")
      (`KismetSystemLibrary.PrintText` (`KismetTextLibrary.Conv_ObjectToText` _player1))
      (`KismetSystemLibrary.PrintText` (`KismetTextLibrary.Conv_ObjectToText` PlayerController)))))

(fn `UserConstructionScript`)